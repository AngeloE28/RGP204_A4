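; BP_HealingCrystals is a crystal pickup that trades the player's other abilities for healing.
; When BP_Player overlaps the Crystal component, it sets the player's CanHeal flag and clears CanShoot and CanDash, with no reset on overlap end.
; Every Tick, LightChanging steps the light intensity up or down, reversing at min and max limits, and applies it to the PointLight for a pulsing glow.
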(event `self.Crystal.OnComponentBeginOverlap`
  (params (OverlappedComponent :type "PrimitiveComponent Object Reference") (OtherActor :type "Actor Object Reference") (OtherComp :type "PrimitiveComponent Object Reference") (OtherBodyIndex :type Integer) (bFromSweep :type Boolean) (SweepResult :type "HitResult Structure (by ref)"))
  ;[1 1 1] Gives the player the ability to heal, in return player loses their other abilities
  (if (== (`GameplayStatics.GetObjectClass` OtherActor) "/Game/ThirdPersonBP/Blueprints/BP_Player.BP_Player_C")
    (bind _asbp_player (cast `/Game/ThirdPersonBP/Blueprints/BP_Player` OtherActor))
    (set `/Game/ThirdPersonBP/Blueprints/BP_Player.canHeal` true _asbp_player)
    (`|ExecutionSequence`
      (:`then_0`
        (set `/Game/ThirdPersonBP/Blueprints/BP_Player.canShoot` false _asbp_player))
      (:`then_1`
        (set `/Game/ThirdPersonBP/Blueprints/BP_Player.canDash` false _asbp_player)))))

(event `self.ReceiveTick`
  (params (DeltaSeconds :type "Float (single-precision)"))
  ;[1 1 1] Runs the light change event
  (`self.LightChanging`)
  (`LightComponent.SetIntensity` (`self.PointLight`) (`self.CurrentLightIntensity`)))

(event `LightChanging`
  ;[1 1 1] Changes light intensity over time
  (`|MultiGate` false true
    (:`Out 0`
      (if (`self.IncreaseIntensity`)
        (set `self.CurrentLightIntensity` (+ (`self.CurrentLightIntensity`) (`self.LightChangeIntensity`)))
        (if (>= (`self.CurrentLightIntensity`) (`self.MaxLightIntensity`))
          (set `self.IncreaseIntensity` false))
        (else
          (set `self.CurrentLightIntensity` (- (`self.CurrentLightIntensity`) (`self.LightChangeIntensity`)))
          (if (<= (`self.CurrentLightIntensity`) (`self.MinLightIntensity`))
            (set `self.IncreaseIntensity` true)))))))

(fn `UserConstructionScript`)