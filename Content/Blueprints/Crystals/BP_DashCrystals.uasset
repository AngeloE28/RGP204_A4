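; Dash crystal pickup that grants BP_Player the dash ability in exchange for shooting and slow-time.
; On overlap with a player lacking dash, it plays a power-change sound and swaps those ability flags.
; Tick animates it: MovemtDash ramps a vertical offset between limits to bob Crystal, and Rotate feeds a wrapping yaw value to spin BlueCrystal.
; Both motions accumulate, since the computed values are applied as per-frame local deltas.
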(event `self.Crystal.OnComponentBeginOverlap`
  (params (OverlappedComponent :type "PrimitiveComponent Object Reference") (OtherActor :type "Actor Object Reference") (OtherComp :type "PrimitiveComponent Object Reference") (OtherBodyIndex :type Integer) (bFromSweep :type Boolean) (SweepResult :type "HitResult Structure (by ref)"))
  ;[1 1 1] Gives the player the ability to dash, in return player loses their other abilities
  (if (== (`GameplayStatics.GetObjectClass` OtherActor) "/Game/Player_BP/Blueprints/BP_Player.BP_Player_C")
    (bind _asbp_player (cast `/Game/Player_BP/Blueprints/BP_Player` OtherActor))
    (if (not (`/Game/Player_BP/Blueprints/BP_Player.canDash` _asbp_player))
      (`AudioComponent.Play` (`self.PowerChangeSoundCue`) 0.0)
      (set `/Game/Player_BP/Blueprints/BP_Player.canDash` true _asbp_player)
      (`|ExecutionSequence`
        (:`then_0`
          (set `/Game/Player_BP/Blueprints/BP_Player.canShoot` false _asbp_player))
        (:`then_1`
          (set `/Game/Player_BP/Blueprints/BP_Player.canSlowTime` false _asbp_player))))))

(event `self.ReceiveTick`
  (params (DeltaSeconds :type "Float (single-precision)"))
  ;[1 1 1] Runs the light change event
  (`|ExecutionSequence`
    (:`then_0`
      (`self.MovemtDash`)
      (`SceneComponent.K2_AddLocalOffset` (`self.Crystal`) (`self.CurrentPos`) false false))
    (:`then_1`
      (`self.Rotate`)
      (`SceneComponent.K2_AddLocalRotation` (`self.BlueCrystal`) (`self.Rotation`) false false))))

(event `MovemtDash`
  ;[1 1 1] Bobs up and down
  (`|MultiGate` false true
    (:`Out 0`
      (if (`self.Move`)
        (bind _output_get (set `self.CurrentPos` (+ (`self.CurrentPos`) (* (`KismetMathLibrary.Vector_Up`) (`self.OffsetChange`)))))
        (set `self.Offset` (.z _output_get))
        (if (>= (`self.Offset`) (`self.MaxOffset`))
          (set `self.Move` false))
        (else
          (bind _output_get_2 (set `self.CurrentPos` (- (`self.CurrentPos`) (* (`KismetMathLibrary.Vector_Up`) (`self.OffsetChange`)))))
          (set `self.Offset` (.z _output_get_2))
          (if (<= (`self.Offset`) (`self.MinOffset`))
            (set `self.Move` true)))))))

(event `Rotate`
  ;[1 1 1] Spins counter clockwise
  (`|MultiGate` false true
    (:`Out 0`
      (bind _output_get (set `self.CurrentRotationIncrement` (- (`self.CurrentRotationIncrement`) (`self.RotationIncrement`))))
      (set `self.Rotation` (`KismetMathLibrary.MakeRotator` 0.0 0.0 _output_get))
      (if (<= (`self.CurrentRotationIncrement`) 0.0)
        (set `self.CurrentRotationIncrement` (`self.MaxRotation`))))))

(fn `UserConstructionScript`)