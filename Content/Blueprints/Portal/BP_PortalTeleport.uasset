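; Portal actor that teleports the player to a linked partner portal when they overlap its mesh.
; Only actors of exactly the BP_Player class trigger it, and they keep their world-space offset from the entry mesh at the destination, with rotation left untouched.
; A CanTeleport flag is cleared on both portals during the jump and restored after a short delay to prevent bouncing straight back.
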(event `self.StaticMeshComponent.OnComponentBeginOverlap`
  (params (OverlappedComponent :type "PrimitiveComponent Object Reference") (OtherActor :type "Actor Object Reference") (OtherComp :type "PrimitiveComponent Object Reference") (OtherBodyIndex :type Integer) (bFromSweep :type Boolean) (SweepResult :type "HitResult Structure (by ref)"))
  ;[1 1 1] Creates a portal system
  (if (== (`GameplayStatics.GetObjectClass` OtherActor) "/Game/Player_BP/Blueprints/BP_Player.BP_Player_C")
    (if (`self.CanTeleport`)
      (set `self.CanTeleport` false)
      (set `/Game/Blueprints/Portal/BP_PortalTeleport.CanTeleport` false (`self.BP_PortalTeleport2`))
      (`self.K2_SetActorLocation` OtherActor (+ (`SceneComponent.K2_GetComponentLocation` (`StaticMeshActor.StaticMeshComponent` (`self.BP_PortalTeleport2`))) (- (`self.K2_GetActorLocation` OtherActor) (`SceneComponent.K2_GetComponentLocation` (`self.StaticMeshComponent`)))) false false)
      (`KismetSystemLibrary.Delay` 0.5)
      (set `/Game/Blueprints/Portal/BP_PortalTeleport.CanTeleport` true (`self.BP_PortalTeleport2`))
      (set `self.CanTeleport` true))))

(fn `UserConstructionScript`)