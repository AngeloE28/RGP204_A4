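; Entrance fountain actor that lights up with fire when the player enters its trigger.
; Overlap by BP_Player sets ActivateLight, which Tick polls to drive the effect.
; A DoOnce spawns fire particles and sounds at five scene points.
; Each tick, five point lights take CurrentIntensity, which climbs by a fixed increment up to MaxIntensity for a gradual fade-in.
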(event `self.ReceiveTick`
  (params (DeltaSeconds :type "Float (single-precision)"))
  ;[1 1 1] Event tick
  (if (`self.ActivateLight`)
    (`|ExecutionSequence`
      (:`then_0`
        ;[1 1 1] Turns on the lights
        (`self.TurnOnLights`))
      (:`then_1`
        (`self.LightIntensity`)))))

(event `SpawnFire`
  (bind _returnvalue (`SceneComponent.K2_GetComponentLocation` (`self.FireSpawnLoc2`)))
  (bind _returnvalue_2 (`SceneComponent.K2_GetComponentLocation` (`self.FireSpawnLoc4`)))
  (bind _returnvalue_3 (`SceneComponent.K2_GetComponentLocation` (`self.FireSpawnLoc`)))
  (bind _returnvalue_4 (`SceneComponent.K2_GetComponentLocation` (`self.FireSpawnLoc5`)))
  (bind _returnvalue_5 (`SceneComponent.K2_GetComponentLocation` (`self.FireSpawnLoc3`)))
  ;[1 1 1] Spawns the fire particle effects with sounds
  (`/Engine/EditorBlueprintResources/StandardMacros.DoOnce` false
    (:`Completed`
      (`|ExecutionSequence`
        (:`then_0`
          (`GameplayStatics.SpawnEmitterAtLocation` "/Game/StarterContent/Particles/P_Fire.P_Fire" _returnvalue_3 (struct :`Pitch` 90.0))
          (`GameplayStatics.PlaySoundAtLocation` "/Game/StarterContent/Audio/Fire01_Cue.Fire01_Cue" _returnvalue_3 (struct) 1.0 1.0 0.0 null null null))
        (:`then_1`
          (`GameplayStatics.SpawnEmitterAtLocation` "/Game/StarterContent/Particles/P_Fire.P_Fire" _returnvalue (struct :`Pitch` 90.0))
          (`GameplayStatics.PlaySoundAtLocation` "/Game/StarterContent/Audio/Fire01_Cue.Fire01_Cue" _returnvalue (struct) 1.0 1.0 0.0 null null null))
        (:`then_2`
          (`GameplayStatics.SpawnEmitterAtLocation` "/Game/StarterContent/Particles/P_Fire.P_Fire" _returnvalue_5 (struct :`Pitch` 90.0))
          (`GameplayStatics.PlaySoundAtLocation` "/Game/StarterContent/Audio/Fire01_Cue.Fire01_Cue" _returnvalue_5 (struct) 1.0 1.0 0.0 null null null))
        (:`then_3`
          (`GameplayStatics.SpawnEmitterAtLocation` "/Game/StarterContent/Particles/P_Fire.P_Fire" _returnvalue_2 (struct :`Pitch` 90.0))
          (`GameplayStatics.PlaySoundAtLocation` "/Game/StarterContent/Audio/Fire01_Cue.Fire01_Cue" _returnvalue_2 (struct) 1.0 1.0 0.0 null null null))
        (:`then_4`
          (`GameplayStatics.SpawnEmitterAtLocation` "/Game/StarterContent/Particles/P_Fire.P_Fire" _returnvalue_4 (struct :`Pitch` 90.0))
          (`GameplayStatics.PlaySoundAtLocation` "/Game/StarterContent/Audio/Fire01_Cue.Fire01_Cue" _returnvalue_4 (struct) 1.0 1.0 0.0 null null null))))))

(event `TurnOnLights`
  (bind _currentintensity (`self.CurrentIntensity`))
  ;[1 1 1] Turns on the lights and spawns the fire with sounds
  (`|ExecutionSequence`
    (:`then_0`
      (`self.SpawnFire`))
    (:`then_1`
      (`LightComponent.SetIntensity` (`Light.LightComponent` (`self.PointLight`)) _currentintensity))
    (:`then_2`
      (`LightComponent.SetIntensity` (`Light.LightComponent` (`self.PointLight2`)) _currentintensity))
    (:`then_3`
      (`LightComponent.SetIntensity` (`Light.LightComponent` (`self.PointLight3`)) _currentintensity))
    (:`then_4`
      (`LightComponent.SetIntensity` (`Light.LightComponent` (`self.PointLight4`)) _currentintensity))
    (:`then_5`
      (`LightComponent.SetIntensity` (`Light.LightComponent` (`self.PointLight5`)) _currentintensity))))

(event `self.TriggerCollider.OnComponentBeginOverlap`
  (params (OverlappedComponent :type "PrimitiveComponent Object Reference") (OtherActor :type "Actor Object Reference") (OtherComp :type "PrimitiveComponent Object Reference") (OtherBodyIndex :type Integer) (bFromSweep :type Boolean) (SweepResult :type "HitResult Structure (by ref)"))
  ;[1 1 1] Triggers event
  (if (== (`GameplayStatics.GetObjectClass` OtherActor) "/Game/Player_BP/Blueprints/BP_Player.BP_Player_C")
    (set `self.ActivateLight` true)))

(event `LightIntensity`
  (bind _maxintensity (`self.MaxIntensity`))
  ;[1 1 1] Sets the light intensity
  (`|MultiGate` false true
    (:`Out 0`
      (bind _output_get (set `self.CurrentIntensity` (+ (`self.CurrentIntensity`) (`self.IntensityIncrement`))))
      (if (> _output_get _maxintensity)
        (set `self.CurrentIntensity` _maxintensity)))))

(fn `UserConstructionScript`)