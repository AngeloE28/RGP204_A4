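; BP_MuralEntrance is a room lighting actor that lights up a mural entrance when the player enters its trigger.
; Overlap by BP_Player sets ActivateLight, which lets Tick drive the lighting from then on.
; A DoOnce spawns fire emitters at two marker locations, while both point lights fade up as a looping MultiGate increments their shared intensity up to a maximum.
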(event `self.ReceiveTick`
  (params (DeltaSeconds :type "Float (single-precision)"))
  ;[1 1 1] Event tick
  (if (`self.ActivateLight`)
    (`|ExecutionSequence`
      (:`then_0`
        ;[1 1 1] Turns on the lights
        (`self.TurnOnLights`))
      (:`then_1`
        (`self.LightIntensity`)))))

(event `SpawnFire`
  ;[1 1 1] Spawns the fire particle effects
  (`/Engine/EditorBlueprintResources/StandardMacros.DoOnce` false
    (:`Completed`
      (`|ExecutionSequence`
        (:`then_0`
          (`GameplayStatics.SpawnEmitterAtLocation` "/Game/StarterContent/Particles/P_Fire.P_Fire" (`SceneComponent.K2_GetComponentLocation` (`self.FireSpawnLoc`)) (struct :`Pitch` 90.0)))
        (:`then_1`
          (`GameplayStatics.SpawnEmitterAtLocation` "/Game/StarterContent/Particles/P_Fire.P_Fire" (`SceneComponent.K2_GetComponentLocation` (`self.FireSpawnLoc2`)) (struct :`Pitch` 90.0)))))))

(event `TurnOnLights`
  (bind _currentintensity (`self.CurrentIntensity`))
  ;[1 1 1] Turns on the lights and spawns the fire
  (`|ExecutionSequence`
    (:`then_0`
      (`self.SpawnFire`))
    (:`then_1`
      (`LightComponent.SetIntensity` (`Light.LightComponent` (`self.PointLight`)) _currentintensity))
    (:`then_2`
      (`LightComponent.SetIntensity` (`Light.LightComponent` (`self.PointLight2`)) _currentintensity))))

(event `self.TriggerCollider.OnComponentBeginOverlap`
  (params (OverlappedComponent :type "PrimitiveComponent Object Reference") (OtherActor :type "Actor Object Reference") (OtherComp :type "PrimitiveComponent Object Reference") (OtherBodyIndex :type Integer) (bFromSweep :type Boolean) (SweepResult :type "HitResult Structure (by ref)"))
  ;[1 1 1] Triggers event
  (if (== (`GameplayStatics.GetObjectClass` OtherActor) "/Game/ThirdPersonBP/Blueprints/BP_Player.BP_Player_C")
    (set `self.ActivateLight` true)))

(event `LightIntensity`
  (bind _maxintensity (`self.MaxIntensity`))
  ;[1 1 1] Sets the light intensity
  (`|MultiGate` false true
    (:`Out 0`
      (bind _output_get (set `self.CurrentIntensity` (+ (`self.CurrentIntensity`) (`self.IntensityIncrement`))))
      (if (> _output_get _maxintensity)
        (set `self.CurrentIntensity` _maxintensity)))))

(fn `UserConstructionScript`)