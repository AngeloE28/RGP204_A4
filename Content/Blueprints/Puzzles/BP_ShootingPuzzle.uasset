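; Shooting puzzle actor that opens a door when the player has all three targets hit at the same time.
; Bullet hits flag each target and swap its materials to lit versions, while a reset delay later clears the flag and restores the original materials.
; Tick polls the flags, plays the MoveDoor level sequence once all are set, then keeps every target lit after completion.
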(event `self.ReceiveTick`
  (params (DeltaSeconds :type "Float (single-precision)"))
  ;[1 1 1] Event tick
  (`|ExecutionSequence`
    (:`then_0`
      ;[1 1 1] Main Events that need to be run
      (`self.OpenDoor`))
    (:`then_1`
      (`self.ResetTargets`))
    (:`then_2`
      (`self.KeepLit`))))

(event `ResetTargets`
  ;[1 1 1] Reset Targets
  (`|ExecutionSequence`
    (:`then_0`
      (if (`self.T1Hit`)
        (`KismetSystemLibrary.Delay` (`self.ResetTimer`))
        (`self.ResetT1Materials`)
        (set `self.T1Hit` false)))
    (:`then_1`
      (if (`self.T2Hit`)
        (`KismetSystemLibrary.Delay` (`self.ResetTimer`))
        (`self.ResetT2Materials`)
        (set `self.T2Hit` false)))
    (:`then_2`
      (if (`self.T3Hit`)
        (`KismetSystemLibrary.Delay` (`self.ResetTimer`))
        (`self.ResetT3Materials`)
        (set `self.T3Hit` false)))))

(event `self.Target1.OnComponentHit`
  (params (HitComponent :type "PrimitiveComponent Object Reference") (OtherActor :type "Actor Object Reference") (OtherComp :type "PrimitiveComponent Object Reference") (NormalImpulse :type "Vector Structure") (Hit :type "HitResult Structure (by ref)"))
  ;[1 1 1] Keeps count how many of each target was hit already, resets its hit state if player took too long
  (if (== (`GameplayStatics.GetObjectClass` OtherActor) "/Game/Blueprints/Player/BP_Bullet.BP_Bullet_C")
    (set `self.T1Hit` true)
    (`self.LightUpT1`)))

(event `self.Target2.OnComponentHit`
  (params (HitComponent :type "PrimitiveComponent Object Reference") (OtherActor :type "Actor Object Reference") (OtherComp :type "PrimitiveComponent Object Reference") (NormalImpulse :type "Vector Structure") (Hit :type "HitResult Structure (by ref)"))
  ;[1 1 1] Keeps count how many of each target was hit already, resets its hit state if player took too long
  (if (== (`GameplayStatics.GetObjectClass` OtherActor) "/Game/Blueprints/Player/BP_Bullet.BP_Bullet_C")
    (set `self.T2Hit` true)
    (`self.LightUpT2`)))

(event `KeepLit`
  ;[1 1 1] Keeps the targets lit
  (if (`self.FinishedPuzzle`)
    (`|ExecutionSequence`
      (:`then_0`
        (`self.LightUpT1`))
      (:`then_1`
        (`self.LightUpT2`))
      (:`then_2`
        (`self.LightUpT3`)))))

(event `self.Target3.OnComponentHit`
  (params (HitComponent :type "PrimitiveComponent Object Reference") (OtherActor :type "Actor Object Reference") (OtherComp :type "PrimitiveComponent Object Reference") (NormalImpulse :type "Vector Structure") (Hit :type "HitResult Structure (by ref)"))
  ;[1 1 1] Keeps count how many of each target was hit already, resets its hit state if player took too long
  (if (== (`GameplayStatics.GetObjectClass` OtherActor) "/Game/Blueprints/Player/BP_Bullet.BP_Bullet_C")
    (set `self.T3Hit` true)
    (`self.LightUpT3`)))

(event `OpenDoor`
  ;[1 1 1] Plays the level sequence
  (if (`self.FinishedPuzzle`)
    _
    (elif (and (== (`self.T1Hit`) true) (== (`self.T2Hit`) true) (== (`self.T3Hit`) true))
      (bind (_outactor _returnvalue) (`LevelSequencePlayer.CreateLevelSequencePlayer` (`self.MoveDoor`)))
      (`MovieSceneSequencePlayer.Play` _returnvalue)
      (set `self.FinishedPuzzle` true)
      (`|ExecutionSequence`
        (:`then_0`
          (set `self.T1Hit` false))
        (:`then_1`
          (set `self.T2Hit` false))
        (:`then_2`
          (set `self.T3Hit` false))))))

(event `ResetT1Materials`
  (bind _target1 (`self.Target1`))
  ;[1 1 1] Reset T1's Materials
  (`|ExecutionSequence`
    (:`then_0`
      (`PrimitiveComponent.SetMaterial` _target1 1 "/Game/Imports/Target/lambert4.lambert4"))
    (:`then_1`
      (`PrimitiveComponent.SetMaterial` _target1 3 "/Game/Imports/Target/lambert5.lambert5"))
    (:`then_2`
      (`PrimitiveComponent.SetMaterial` _target1 4 "/Game/Imports/Target/lambert6.lambert6"))))

(event `ResetT2Materials`
  (bind _target2 (`self.Target2`))
  ;[1 1 1] Reset T2's Materials
  (`|ExecutionSequence`
    (:`then_0`
      (`PrimitiveComponent.SetMaterial` _target2 1 "/Game/Imports/Target/lambert4.lambert4"))
    (:`then_1`
      (`PrimitiveComponent.SetMaterial` _target2 3 "/Game/Imports/Target/lambert5.lambert5"))
    (:`then_2`
      (`PrimitiveComponent.SetMaterial` _target2 4 "/Game/Imports/Target/lambert6.lambert6"))))

(event `ResetT3Materials`
  (bind _target3 (`self.Target3`))
  ;[1 1 1] Reset T3's Materials
  (`|ExecutionSequence`
    (:`then_0`
      (`PrimitiveComponent.SetMaterial` _target3 1 "/Game/Imports/Target/lambert4.lambert4"))
    (:`then_1`
      (`PrimitiveComponent.SetMaterial` _target3 3 "/Game/Imports/Target/lambert5.lambert5"))
    (:`then_2`
      (`PrimitiveComponent.SetMaterial` _target3 4 "/Game/Imports/Target/lambert6.lambert6"))))

(event `LightUpT2`
  (bind _target2 (`self.Target2`))
  ;[1 1 1] Lights up T2
  (`|ExecutionSequence`
    (:`then_0`
      (`PrimitiveComponent.SetMaterial` _target2 1 "/Game/Materials/E_Lambert.E_Lambert"))
    (:`then_1`
      (`PrimitiveComponent.SetMaterial` _target2 3 "/Game/Materials/E_Blue.E_Blue"))
    (:`then_2`
      (`PrimitiveComponent.SetMaterial` _target2 4 "/Game/Materials/E_Red.E_Red"))))

(event `LightUpT3`
  (bind _target3 (`self.Target3`))
  ;[1 1 1] Lights up T3
  (`|ExecutionSequence`
    (:`then_0`
      (`PrimitiveComponent.SetMaterial` _target3 1 "/Game/Materials/E_Lambert.E_Lambert"))
    (:`then_1`
      (`PrimitiveComponent.SetMaterial` _target3 3 "/Game/Materials/E_Blue.E_Blue"))
    (:`then_2`
      (`PrimitiveComponent.SetMaterial` _target3 4 "/Game/Materials/E_Red.E_Red"))))

(event `LightUpT1`
  (bind _target1 (`self.Target1`))
  ;[1 1 1] Lights up T1
  (`|ExecutionSequence`
    (:`then_0`
      (`PrimitiveComponent.SetMaterial` _target1 1 "/Game/Materials/E_Lambert.E_Lambert"))
    (:`then_1`
      (`PrimitiveComponent.SetMaterial` _target1 3 "/Game/Materials/E_Blue.E_Blue"))
    (:`then_2`
      (`PrimitiveComponent.SetMaterial` _target1 4 "/Game/Materials/E_Red.E_Red"))))

(fn `UserConstructionScript`)