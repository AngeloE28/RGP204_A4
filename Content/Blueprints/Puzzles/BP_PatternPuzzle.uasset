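; Memory puzzle where the player hits five coloured crystals in a random order, shuffled at BeginPlay and flashed as a hint.
; A player overlap starts Tick-driven logic that briefly raises barriers, plays the hint and checks recorded unique hits against the order.
; Correct hits stay lit, while a wrong one clears progress and re-arms the hint.
; Completion plays a crystal-spin sequence, lights the statue and spawns a gold shower.
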(event `self.ReceiveTick`
  (params (DeltaSeconds :type "Float (single-precision)"))
  ;[1 1 1] Event tick
  ;[1 1 1] Runs the events if player has triggered it
  (if (`self.StartPuzzle`)
    (`|ExecutionSequence`
      (:`then_0`
        ;[1 1 1] Pattern hint event
        (`/Engine/EditorBlueprintResources/StandardMacros.DoOnce` false :!label _label
          (:`Completed`
            (`self.EnableBarriers`)
            (`KismetSystemLibrary.Delay` (`self.PuzzleDelay`))
            (`self.ChangeColourPatternHint`)
            (`self.DisableBarriers`))))
      (:`then_1`
        (if (`self.LoopFin`)
          (if (`self.PuzzleFailed`)
            (goto _label :!via `Reset`))))
      (:`then_2`
        ;[1 1 1] Player interactions
        (`self.PatternPuzzleInteraction`)
        (`self.PuzzleFinished`))
      (:`then_3`
        (if (not (`self.PuzzleFailed`))
          (`self.LightUpHitCrystals`)))
      (:`then_4`
        ;[1 1 1] Finished event
        (if (`self.PuzzleFin`)
          (`/Engine/EditorBlueprintResources/StandardMacros.DoOnce` false
            (:`Completed`
              (`self.SpinCrystal`))))))))

(event `self.ReceiveBeginPlay`
  ;[1 1 1] Begin play
  ;[1 1 1] Runs the crystal order generator
  (`self.GenerateCrystalOrder`))

(event `self.Blue.OnComponentHit`
  (params (HitComponent :type "PrimitiveComponent Object Reference") (OtherActor :type "Actor Object Reference") (OtherComp :type "PrimitiveComponent Object Reference") (NormalImpulse :type "Vector Structure") (Hit :type "HitResult Structure (by ref)"))
  ;[1 1 1] Adds a crystal to the array if it has been hit, only unique values are added
  (`KismetArrayLibrary.Array_AddUnique` (`self.CrystalArr`) (`self.Blue`)))

(event `PuzzleFinished`
  ;[1 1 1] Check if puzzle is finished and runs the finished event
  (if (== (`KismetArrayLibrary.Array_Length` (`self.CrystalArr`)) (`KismetArrayLibrary.Array_Length` (`self.CrystalOrderArr`)))
    (if (`KismetArrayLibrary.Array_Identical` (`self.CrystalOrderArr`) (`self.CrystalArr`))
      (set `self.PuzzleFin` true))))

(event `PatternPuzzleInteraction`
  ;[1 1 1] Pattern puzzle interaction
  (set `self.PuzzleFailed` false)
  (for (_array_element _array_index) (`self.CrystalArr`)
    (if (== (`|GetArrayItem` (`self.CrystalOrderArr`) _array_index) _array_element)
      (set `self.PuzzleFailed` false)
      (else
        (`|ExecutionSequence`
          (:`then_0`
            (set `self.PuzzleFailed` true)
            (`self.ResetCrystalMaterials`)
            (`KismetArrayLibrary.Array_Clear` (`self.CrystalArr`)))
          (:`then_1`
            (break)))))))

(event `self.Yellow.OnComponentHit`
  (params (HitComponent :type "PrimitiveComponent Object Reference") (OtherActor :type "Actor Object Reference") (OtherComp :type "PrimitiveComponent Object Reference") (NormalImpulse :type "Vector Structure") (Hit :type "HitResult Structure (by ref)"))
  ;[1 1 1] Adds a crystal to the array if it has been hit, only unique values are added
  (`KismetArrayLibrary.Array_AddUnique` (`self.CrystalArr`) (`self.Yellow`)))

(event `self.Turquoise.OnComponentHit`
  (params (HitComponent :type "PrimitiveComponent Object Reference") (OtherActor :type "Actor Object Reference") (OtherComp :type "PrimitiveComponent Object Reference") (NormalImpulse :type "Vector Structure") (Hit :type "HitResult Structure (by ref)"))
  ;[1 1 1] Adds a crystal to the array if it has been hit, only unique values are added
  (`KismetArrayLibrary.Array_AddUnique` (`self.CrystalArr`) (`self.Turquoise`)))

(event `self.Purple.OnComponentHit`
  (params (HitComponent :type "PrimitiveComponent Object Reference") (OtherActor :type "Actor Object Reference") (OtherComp :type "PrimitiveComponent Object Reference") (NormalImpulse :type "Vector Structure") (Hit :type "HitResult Structure (by ref)"))
  ;[1 1 1] Adds a crystal to the array if it has been hit, only unique values are added
  (`KismetArrayLibrary.Array_AddUnique` (`self.CrystalArr`) (`self.Purple`)))

(event `GenerateCrystalOrder`
  ;[1 1 1] Generates a random order for the crystals to be shot
  (bind _output_get (set `self.CrystalOrderArr` (`|MakeArray` (`self.Blue`) (`self.Yellow`) (`self.Turquoise`) (`self.Purple`) (`self.Red`))))
  (`KismetArrayLibrary.Array_Shuffle` _output_get))

(event `EnableBarriers`
  ;[1 1 1] Enables the barriers so player can't hit while looking at the pattern
  (`PrimitiveComponent.SetCollisionProfileName` (`self.BlueBarrier`) "BlockAll" true)
  (`PrimitiveComponent.SetCollisionProfileName` (`self.YellowBarrier`) "BlockAll" true)
  (`PrimitiveComponent.SetCollisionProfileName` (`self.TurquoiseBarrier`) "BlockAll" true)
  (`PrimitiveComponent.SetCollisionProfileName` (`self.PurpleBarrier`) "BlockAll" true)
  (`PrimitiveComponent.SetCollisionProfileName` (`self.RedBarrier`) "BlockAll" true))

(event `DisableBarriers`
  ;[1 1 1] Disables barriers so player can hit crystals now
  (`PrimitiveComponent.SetCollisionProfileName` (`self.BlueBarrier`) "NoCollision" true)
  (`PrimitiveComponent.SetCollisionProfileName` (`self.YellowBarrier`) "NoCollision" true)
  (`PrimitiveComponent.SetCollisionProfileName` (`self.TurquoiseBarrier`) "NoCollision" true)
  (`PrimitiveComponent.SetCollisionProfileName` (`self.PurpleBarrier`) "NoCollision" true)
  (`PrimitiveComponent.SetCollisionProfileName` (`self.RedBarrier`) "NoCollision" true))

(event `SpinCrystal`
  ;[1 1 1] Plays the level sequence
  (bind (_outactor _returnvalue) (`LevelSequencePlayer.CreateLevelSequencePlayer` (`self.CrystalSpinSpin`)))
  (`MovieSceneSequencePlayer.Play` _returnvalue)
  (`self.LightUpStatue`)
  (`NiagaraFunctionLibrary.SpawnSystemAtLocation` "/Game/Effects/GoldShower.GoldShower" (`SceneComponent.K2_GetComponentLocation` (`self.FountainSpawn`)) (struct :`Pitch` 15.0)))

(event `self.Red.OnComponentHit`
  (params (HitComponent :type "PrimitiveComponent Object Reference") (OtherActor :type "Actor Object Reference") (OtherComp :type "PrimitiveComponent Object Reference") (NormalImpulse :type "Vector Structure") (Hit :type "HitResult Structure (by ref)"))
  ;[1 1 1] Adds a crystal to the array if it has been hit, only unique values are added
  (`KismetArrayLibrary.Array_AddUnique` (`self.CrystalArr`) (`self.Red`)))

(event `ChangeColourPatternHint`
  ;[1 1 1] Shows the pattern the player has to hit, by changing the material and resetting it back to its default colour
  (bind _arrayelement (`/Game/Blueprints/CustomMacros/BPM_MacroLibrary.For Each Loop with Delay` (`self.CrystalOrderArr`) (`self.ResetMatDelay`))
    (:`LoopBody`
      (set `self.LoopFin` false)
      (`|ExecutionSequence`
        (:`then_0`
          (if (== _arrayelement (`self.Blue`))
            (`self.LightUpBlueCrystal`)
            (`KismetSystemLibrary.Delay` (`self.ResetMatDelay`))
            (`self.ResetBlueCrystalMat`)))
        (:`then_1`
          (if (== _arrayelement (`self.Yellow`))
            (`self.LightUpYellowCrystal`)
            (`KismetSystemLibrary.Delay` (`self.ResetMatDelay`))
            (`self.ResetYellowCrystalMat`)))
        (:`then_2`
          (if (== _arrayelement (`self.Turquoise`))
            (`self.LightUpTurquoiseCrystal`)
            (`KismetSystemLibrary.Delay` (`self.ResetMatDelay`))
            (`self.ResetTurquoiseCrystalMat`)))
        (:`then_3`
          (if (== _arrayelement (`self.Purple`))
            (`self.LightUpPurpleCrystal`)
            (`KismetSystemLibrary.Delay` (`self.ResetMatDelay`))
            (`self.ResetPurpleCrystalMat`)))
        (:`then_4`
          (if (== _arrayelement (`self.Red`))
            (`self.LightUpRedCrystal`)
            (`KismetSystemLibrary.Delay` (`self.ResetMatDelay`))
            (`self.ResetRedCrystalMat`)))))
    (:`Complete`
      (set `self.LoopFin` true))))

(event `LightUpHitCrystals`
  ;[1 1 1] Light up crystals that were hit
  (for _array_element (`self.CrystalArr`)
    (`|ExecutionSequence`
      (:`then_0`
        (if (== _array_element (`self.Blue`))
          (`self.LightUpBlueCrystal`)))
      (:`then_1`
        (if (== _array_element (`self.Yellow`))
          (`self.LightUpYellowCrystal`)))
      (:`then_2`
        (if (== _array_element (`self.Turquoise`))
          (`self.LightUpTurquoiseCrystal`)))
      (:`then_3`
        (if (== _array_element (`self.Purple`))
          (`self.LightUpPurpleCrystal`)))
      (:`then_4`
        (if (== _array_element (`self.Red`))
          (`self.LightUpRedCrystal`))))))

(event `LightUpStatue`
  ;[1 1 1] Lights up the statue
  (`|ExecutionSequence`
    (:`then_0`
      (`PrimitiveComponent.SetMaterial` (`StaticMeshActor.StaticMeshComponent` (`self.SexySword`)) 1 "/Game/Materials/LavaMat_Inst.LavaMat_Inst"))
    (:`then_1`
      (`PrimitiveComponent.SetMaterial` (`StaticMeshActor.StaticMeshComponent` (`self.SexyStatue`)) 2 "/Game/Materials/E_Mats/E_Eyes.E_Eyes"))))

(event `ResetCrystalMaterials`
  ;[1 1 1] Resets each crystal materials to default when the player fails the puzzle
  (for _array_element (`self.CrystalArr`)
    (`|ExecutionSequence`
      (:`then_0`
        (if (== _array_element (`self.Blue`))
          (`self.ResetBlueCrystalMat`)))
      (:`then_1`
        (if (== _array_element (`self.Yellow`))
          (`self.ResetYellowCrystalMat`)))
      (:`then_2`
        (if (== _array_element (`self.Turquoise`))
          (`self.ResetTurquoiseCrystalMat`)))
      (:`then_3`
        (if (== _array_element (`self.Purple`))
          (`self.ResetPurpleCrystalMat`)))
      (:`then_4`
        (if (== _array_element (`self.Red`))
          (`self.ResetRedCrystalMat`))))))

(event `LightUpBlueCrystal`
  ;[1 1 1] Lights up blue crystal
  (`PrimitiveComponent.SetMaterial` (`self.Blue`) 0 "/Game/Materials/E_Mats/E_BlueCrystal_Inst.E_BlueCrystal_Inst"))

(event `ResetBlueCrystalMat`
  ;[1 1 1] Resets the blue crystal material
  (`PrimitiveComponent.SetMaterial` (`self.Blue`) 0 "/Game/Materials/GhostTrail/Blue_CrystalMat_Inst.Blue_CrystalMat_Inst"))

(event `ResetYellowCrystalMat`
  ;[1 1 1] Resets the yellow crystal material
  (`PrimitiveComponent.SetMaterial` (`self.Yellow`) 0 "/Game/Materials/GhostTrail/Yellow_CrystalMat_Inst_.Yellow_CrystalMat_Inst_"))

(event `LightUpYellowCrystal`
  ;[1 1 1] Light up yellow crystal
  (`PrimitiveComponent.SetMaterial` (`self.Yellow`) 0 "/Game/Materials/E_Mats/E_YellowCrystal_Inst.E_YellowCrystal_Inst"))

(event `ResetTurquoiseCrystalMat`
  ;[1 1 1] Resets the turquoise material
  (`PrimitiveComponent.SetMaterial` (`self.Turquoise`) 0 "/Game/Materials/GhostTrail/Turquoise_CrystalMat_Inst.Turquoise_CrystalMat_Inst"))

(event `LightUpTurquoiseCrystal`
  ;[1 1 1] Lights up the turquoise crystal
  (`PrimitiveComponent.SetMaterial` (`self.Turquoise`) 0 "/Game/Materials/E_Mats/E_TurquoiseCrystal_Inst.E_TurquoiseCrystal_Inst"))

(event `ResetPurpleCrystalMat`
  ;[1 1 1] Resets the purple crystal
  (`PrimitiveComponent.SetMaterial` (`self.Purple`) 0 "/Game/Materials/GhostTrail/Purple_CrystalMat_Inst.Purple_CrystalMat_Inst"))

(event `LightUpPurpleCrystal`
  ;[1 1 1] Lights up the purple crystal
  (`PrimitiveComponent.SetMaterial` (`self.Purple`) 0 "/Game/Materials/E_Mats/E_PurpleCrystal_Inst.E_PurpleCrystal_Inst"))

(event `LightUpRedCrystal`
  ;[1 1 1] Lights up red crystal
  (`PrimitiveComponent.SetMaterial` (`self.Red`) 0 "/Game/Materials/E_Mats/E_RedCrystal_Inst.E_RedCrystal_Inst"))

(event `ResetRedCrystalMat`
  ;[1 1 1] Resets the red crystal material
  (`PrimitiveComponent.SetMaterial` (`self.Red`) 0 "/Game/Materials/GhostTrail/Red_CrystalMat_Inst.Red_CrystalMat_Inst"))

(event `self.ColliderTrigger.OnComponentBeginOverlap`
  (params (OverlappedComponent :type "PrimitiveComponent Object Reference") (OtherActor :type "Actor Object Reference") (OtherComp :type "PrimitiveComponent Object Reference") (OtherBodyIndex :type Integer) (bFromSweep :type Boolean) (SweepResult :type "HitResult Structure (by ref)"))
  ;[1 1 1] Trigger puzzle events
  (if (== (`GameplayStatics.GetObjectClass` OtherActor) "/Game/ThirdPersonBP/Blueprints/BP_Player.BP_Player_C")
    (`KismetSystemLibrary.Delay` (`self.StartPuzzleDelay`))
    (set `self.StartPuzzle` true)))

(fn `UserConstructionScript`)