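; BP_LockPuzzle is a lock puzzle actor that opens a door and lights up a statue once its key arrives.
; An overlap on its collider sets a key flag without checking which actor entered.
; Tick polls that flag, then plays the MoveDoor2 level sequence once and swaps material slots on the referenced sword and statue meshes.
; A finished flag keeps the puzzle from firing again.
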(event `self.ReceiveTick`
  (params (DeltaSeconds :type "Float (single-precision)"))
  ;[1 1 1] Event Tick
  (`self.OpenDoor`))

(event `self.Collider.OnComponentBeginOverlap`
  (params (OverlappedComponent :type "PrimitiveComponent Object Reference") (OtherActor :type "Actor Object Reference") (OtherComp :type "PrimitiveComponent Object Reference") (OtherBodyIndex :type Integer) (bFromSweep :type Boolean) (SweepResult :type "HitResult Structure (by ref)"))
  ;[1 1 1] The key was received
  (set `self.GotKey` true))

(event `OpenDoor`
  ;[1 1 1] Plays the level sequence
  (if (`self.FinishedPuzzle`)
    _
    (elif (`self.GotKey`)
      (bind (_outactor _returnvalue) (`LevelSequencePlayer.CreateLevelSequencePlayer` (`self.MoveDoor2`)))
      (`MovieSceneSequencePlayer.Play` _returnvalue)
      (`self.LightUp Statue`)
      (set `self.GotKey` false)
      (set `self.FinishedPuzzle` true))))

(event `LightUp Statue`
  ;[1 1 1] Lights up the statue
  (`|ExecutionSequence`
    (:`then_0`
      (`PrimitiveComponent.SetMaterial` (`StaticMeshActor.StaticMeshComponent` (`self.SexySword`)) 1 "/Game/Materials/LavaMat_Inst.LavaMat_Inst"))
    (:`then_1`
      (`PrimitiveComponent.SetMaterial` (`StaticMeshActor.StaticMeshComponent` (`self.SexyStatue`)) 2 "/Game/Materials/E_Eyes.E_Eyes"))))

(fn `UserConstructionScript`)