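; Chess board for the mural puzzle, solved when eight specific black and white pieces rest on their matching squares.
; Per-piece collider overlaps set flags and references, which Tick polls to detect completion and make the player drop the held object after a delay.
; Completion plays a statue sequence once, lights up the statue, spawns a gold fountain and goat piece, then keeps snapping piece rotations to their colliders every tick.
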(event `self.ReceiveBeginPlay`
  ;[1 1 1] Begin play
  ;[1 1 1] Gets the player
  (bind _returnvalue (`GameplayStatics.GetActorOfClass` "/Game/ThirdPersonBP/Blueprints/BP_Player.BP_Player_C"))
  (set `self.Player` _returnvalue))

(event `LightUpStatue`
  ;[1 1 1] Lights up the statue
  (`|ExecutionSequence`
    (:`then_0`
      (`PrimitiveComponent.SetMaterial` (`StaticMeshActor.StaticMeshComponent` (`self.SexySword`)) 1 "/Game/Materials/LavaMat_Inst.LavaMat_Inst"))
    (:`then_1`
      (`PrimitiveComponent.SetMaterial` (`StaticMeshActor.StaticMeshComponent` (`self.SexyStatue`)) 2 "/Game/Materials/E_Mats/E_Eyes.E_Eyes"))))

(event `PuzzleFinished`
  ;[1 1 1] Controls if the puzzle is finished or not
  (if (and (== (`self.GotBlackKnight`) true) (== (`self.GotBlackPawn`) true) (== (`self.GotBlackPawn2`) true) (== (`self.GotBlackKing`) true) (== (`self.GotWhiteQueen`) true) (== (`self.GotWhiteKing`) true) (== (`self.GotWhiteRook`) true) (== (`self.GotWhiteBishop`) true))
    (set `self.PuzzleFin` true)
    (`/Engine/EditorBlueprintResources/StandardMacros.DoOnce` false
      (:`Completed`
        (`KismetSystemLibrary.Delay` (`self.DropDelay`))
        (`/Game/ThirdPersonBP/Blueprints/BP_Player.DropPhysicsObject` (`self.Player`))))))

(event `SpawnFountainAndGoatPiece`
  ;[1 1 1] Spawns the effect and the goat piece
  (`NiagaraFunctionLibrary.SpawnSystemAtLocation` "/Game/Effects/BeegGoldShower.BeegGoldShower" (`SceneComponent.K2_GetComponentLocation` (`self.FountainSpawn`)) (struct))
  (`|SpawnActorFromClass` "/Game/Blueprints/Puzzles/TablePuzzle/BP_GoatPiece.BP_GoatPiece_C" (`KismetMathLibrary.MakeTransform` (`SceneComponent.K2_GetComponentLocation` (`self.GoatPieceSpawn`)) (struct) (2.2 2.2 2.2)) "AlwaysSpawn" "OverrideRootScale" null null))

(event `self.ReceiveTick`
  (params (DeltaSeconds :type "Float (single-precision)"))
  ;[1 1 1] Event tick
  (`|ExecutionSequence`
    (:`then_0`
      ;[1 1 1] Major mural puzzle events
      (`self.PuzzleFinished`))
    (:`then_1`
      (`self.PlayStatueTing`))
    (:`then_2`
      (`self.SetAllPiecesRotation`))))

(event `SetAllPiecesRotation`
  ;[1 1 1] Sets the rotation of all the pieces
  (if (`self.SetRots`)
    (`|ExecutionSequence`
      (:`then_0`
        (`self.SetBlackPiecesRotation`))
      (:`then_1`
        (`self.SetWhitePiecesRotation`)))))

(event `self.BlackKnightCollider.OnComponentBeginOverlap`
  (params (OverlappedComponent :type "PrimitiveComponent Object Reference") (OtherActor :type "Actor Object Reference") (OtherComp :type "PrimitiveComponent Object Reference") (OtherBodyIndex :type Integer) (bFromSweep :type Boolean) (SweepResult :type "HitResult Structure (by ref)"))
  ;[1 1 1] Chess piece has entered the right spot
  (if (== (`GameplayStatics.GetObjectClass` OtherActor) "/Game/Blueprints/Puzzles/MuralPuzzle/BlackPieces/BP_BlackKnight.BP_BlackKnight_C")
    (set `self.GotBlackKnight` true)
    (set `self.BlackKnight` OtherActor)))

(event `self.BlackKnightCollider.OnComponentEndOverlap`
  (params (OverlappedComponent :type "PrimitiveComponent Object Reference") (OtherActor :type "Actor Object Reference") (OtherComp :type "PrimitiveComponent Object Reference") (OtherBodyIndex :type Integer))
  ;[1 1 1] Chess piece left its spot
  (if (== (`GameplayStatics.GetObjectClass` OtherActor) "/Game/Blueprints/Puzzles/MuralPuzzle/BlackPieces/BP_BlackKnight.BP_BlackKnight_C")
    (set `self.GotBlackKnight` false)
    (set `self.BlackKnight` null)))

(event `self.BlackPawnCollider.OnComponentBeginOverlap`
  (params (OverlappedComponent :type "PrimitiveComponent Object Reference") (OtherActor :type "Actor Object Reference") (OtherComp :type "PrimitiveComponent Object Reference") (OtherBodyIndex :type Integer) (bFromSweep :type Boolean) (SweepResult :type "HitResult Structure (by ref)"))
  ;[1 1 1] Chess piece has entered the right spot
  (if (== (`GameplayStatics.GetObjectClass` OtherActor) "/Game/Blueprints/Puzzles/MuralPuzzle/BlackPieces/BP_BlackPawn.BP_BlackPawn_C")
    (set `self.GotBlackPawn` true)
    (set `self.BlackPawn` OtherActor)))

(event `self.BlackPawnCollider.OnComponentEndOverlap`
  (params (OverlappedComponent :type "PrimitiveComponent Object Reference") (OtherActor :type "Actor Object Reference") (OtherComp :type "PrimitiveComponent Object Reference") (OtherBodyIndex :type Integer))
  ;[1 1 1] Chess piece left its spot
  (if (== (`GameplayStatics.GetObjectClass` OtherActor) "/Game/Blueprints/Puzzles/MuralPuzzle/BlackPieces/BP_BlackPawn.BP_BlackPawn_C")
    (set `self.GotBlackPawn` false)
    (set `self.BlackPawn` null)))

(event `PlayStatueTing`
  ;[1 1 1] Plays the level sequence
  (if (`self.SequencePlayed`)
    _
    (elif (`self.PuzzleFin`)
      (bind (_outactor _returnvalue) (`LevelSequencePlayer.CreateLevelSequencePlayer` (`self.StatueTing`)))
      (`MovieSceneSequencePlayer.Play` _returnvalue)
      (`self.LightUpStatue`)
      (`self.SpawnFountainAndGoatPiece`)
      (set `self.PuzzleFin` false)
      (set `self.SequencePlayed` true)
      (set `self.SetRots` true))))

(event `self.BlackPawnCollider2.OnComponentBeginOverlap`
  (params (OverlappedComponent :type "PrimitiveComponent Object Reference") (OtherActor :type "Actor Object Reference") (OtherComp :type "PrimitiveComponent Object Reference") (OtherBodyIndex :type Integer) (bFromSweep :type Boolean) (SweepResult :type "HitResult Structure (by ref)"))
  ;[1 1 1] Chess piece has entered the right spot
  (if (== (`GameplayStatics.GetObjectClass` OtherActor) "/Game/Blueprints/Puzzles/MuralPuzzle/BlackPieces/BP_BlackPawn.BP_BlackPawn_C")
    (set `self.GotBlackPawn2` true)
    (set `self.BlackPawn2` OtherActor)))

(event `self.BlackPawnCollider2.OnComponentEndOverlap`
  (params (OverlappedComponent :type "PrimitiveComponent Object Reference") (OtherActor :type "Actor Object Reference") (OtherComp :type "PrimitiveComponent Object Reference") (OtherBodyIndex :type Integer))
  ;[1 1 1] Chess piece left its spot
  (if (== (`GameplayStatics.GetObjectClass` OtherActor) "/Game/Blueprints/Puzzles/MuralPuzzle/BlackPieces/BP_BlackPawn.BP_BlackPawn_C")
    (set `self.GotBlackPawn2` false)
    (set `self.BlackPawn2` null)))

(event `self.BlackKingCollider.OnComponentBeginOverlap`
  (params (OverlappedComponent :type "PrimitiveComponent Object Reference") (OtherActor :type "Actor Object Reference") (OtherComp :type "PrimitiveComponent Object Reference") (OtherBodyIndex :type Integer) (bFromSweep :type Boolean) (SweepResult :type "HitResult Structure (by ref)"))
  ;[1 1 1] Chess piece has entered the right spot
  (if (== (`GameplayStatics.GetObjectClass` OtherActor) "/Game/Blueprints/Puzzles/MuralPuzzle/BlackPieces/BP_BlackKing.BP_BlackKing_C")
    (set `self.GotBlackKing` true)
    (set `self.BlackKing` OtherActor)))

(event `self.BlackKingCollider.OnComponentEndOverlap`
  (params (OverlappedComponent :type "PrimitiveComponent Object Reference") (OtherActor :type "Actor Object Reference") (OtherComp :type "PrimitiveComponent Object Reference") (OtherBodyIndex :type Integer))
  ;[1 1 1] Chess piece left its spot
  (if (== (`GameplayStatics.GetObjectClass` OtherActor) "/Game/Blueprints/Puzzles/MuralPuzzle/BlackPieces/BP_BlackKing.BP_BlackKing_C")
    (set `self.GotBlackKing` false)
    (set `self.BlackKing` null)))

(event `SetWhitePiecesRotation`
  ;[1 1 1] Sets the white pieces rotation
  (`|ExecutionSequence`
    (:`then_0`
      ;[1 1 1] White Queen rotation
      (`self.K2_SetActorRotation` (`self.WhiteQueen`) (`SceneComponent.K2_GetComponentRotation` (`self.WhiteQueenCollider`)) false))
    (:`then_1`
      ;[1 1 1] White King rotation
      (`self.K2_SetActorRotation` (`self.WhiteKing`) (`SceneComponent.K2_GetComponentRotation` (`self.WhiteKingCollider`)) false))
    (:`then_2`
      ;[1 1 1] White Rook rotation
      (`self.K2_SetActorRotation` (`self.WhiteRook`) (`SceneComponent.K2_GetComponentRotation` (`self.WhiteRookCollider`)) false))
    (:`then_3`
      ;[1 1 1] White Bishop rotation
      (`self.K2_SetActorRotation` (`self.WhiteBishop`) (`SceneComponent.K2_GetComponentRotation` (`self.WhiteBishopCollider`)) false))))

(event `SetBlackPiecesRotation`
  ;[1 1 1] Sets the black pieces rotations
  (`|ExecutionSequence`
    (:`then_0`
      ;[1 1 1] Black Knight rotation
      (`self.K2_SetActorRotation` (`self.BlackKnight`) (`SceneComponent.K2_GetComponentRotation` (`self.BlackKnightCollider`)) false))
    (:`then_1`
      ;[1 1 1] Black Pawn 1 rotation
      (`self.K2_SetActorRotation` (`self.BlackPawn`) (`SceneComponent.K2_GetComponentRotation` (`self.BlackPawnCollider`)) false))
    (:`then_2`
      ;[1 1 1] Black Pawn 2 rotation
      (`self.K2_SetActorRotation` (`self.BlackPawn2`) (`SceneComponent.K2_GetComponentRotation` (`self.BlackPawnCollider2`)) false))
    (:`then_3`
      ;[1 1 1] Black King rotation
      (`self.K2_SetActorRotation` (`self.BlackKing`) (`SceneComponent.K2_GetComponentRotation` (`self.BlackKingCollider`)) false))))

(event `self.WhiteQueenCollider.OnComponentBeginOverlap`
  (params (OverlappedComponent :type "PrimitiveComponent Object Reference") (OtherActor :type "Actor Object Reference") (OtherComp :type "PrimitiveComponent Object Reference") (OtherBodyIndex :type Integer) (bFromSweep :type Boolean) (SweepResult :type "HitResult Structure (by ref)"))
  ;[1 1 1] Chess piece has entered the right spot
  (if (== (`GameplayStatics.GetObjectClass` OtherActor) "/Game/Blueprints/Puzzles/MuralPuzzle/WhitePieces/BP_WhiteQueen.BP_WhiteQueen_C")
    (set `self.GotWhiteQueen` true)
    (set `self.WhiteQueen` OtherActor)))

(event `self.WhiteQueenCollider.OnComponentEndOverlap`
  (params (OverlappedComponent :type "PrimitiveComponent Object Reference") (OtherActor :type "Actor Object Reference") (OtherComp :type "PrimitiveComponent Object Reference") (OtherBodyIndex :type Integer))
  ;[1 1 1] Chess piece left its spot
  (if (== (`GameplayStatics.GetObjectClass` OtherActor) "/Game/Blueprints/Puzzles/MuralPuzzle/WhitePieces/BP_WhiteQueen.BP_WhiteQueen_C")
    (set `self.GotWhiteQueen` false)
    (set `self.WhiteQueen` null)))

(event `self.WhiteKingCollider.OnComponentBeginOverlap`
  (params (OverlappedComponent :type "PrimitiveComponent Object Reference") (OtherActor :type "Actor Object Reference") (OtherComp :type "PrimitiveComponent Object Reference") (OtherBodyIndex :type Integer) (bFromSweep :type Boolean) (SweepResult :type "HitResult Structure (by ref)"))
  ;[1 1 1] Chess piece has entered the right spot
  (if (== (`GameplayStatics.GetObjectClass` OtherActor) "/Game/Blueprints/Puzzles/MuralPuzzle/WhitePieces/BP_WhiteKing.BP_WhiteKing_C")
    (set `self.GotWhiteKing` true)
    (set `self.WhiteKing` OtherActor)))

(event `self.WhiteKingCollider.OnComponentEndOverlap`
  (params (OverlappedComponent :type "PrimitiveComponent Object Reference") (OtherActor :type "Actor Object Reference") (OtherComp :type "PrimitiveComponent Object Reference") (OtherBodyIndex :type Integer))
  ;[1 1 1] Chess piece left its spot
  (if (== (`GameplayStatics.GetObjectClass` OtherActor) "/Game/Blueprints/Puzzles/MuralPuzzle/WhitePieces/BP_WhiteKing.BP_WhiteKing_C")
    (set `self.GotWhiteKing` false)
    (set `self.WhiteKing` null)))

(event `self.WhiteRookCollider.OnComponentBeginOverlap`
  (params (OverlappedComponent :type "PrimitiveComponent Object Reference") (OtherActor :type "Actor Object Reference") (OtherComp :type "PrimitiveComponent Object Reference") (OtherBodyIndex :type Integer) (bFromSweep :type Boolean) (SweepResult :type "HitResult Structure (by ref)"))
  ;[1 1 1] Chess piece has entered the right spot
  (if (== (`GameplayStatics.GetObjectClass` OtherActor) "/Game/Blueprints/Puzzles/MuralPuzzle/WhitePieces/BP_WhiteRook.BP_WhiteRook_C")
    (set `self.GotWhiteRook` true)
    (set `self.WhiteRook` OtherActor)))

(event `self.WhiteRookCollider.OnComponentEndOverlap`
  (params (OverlappedComponent :type "PrimitiveComponent Object Reference") (OtherActor :type "Actor Object Reference") (OtherComp :type "PrimitiveComponent Object Reference") (OtherBodyIndex :type Integer))
  ;[1 1 1] Chess piece left its spot
  (if (== (`GameplayStatics.GetObjectClass` OtherActor) "/Game/Blueprints/Puzzles/MuralPuzzle/WhitePieces/BP_WhiteRook.BP_WhiteRook_C")
    (set `self.GotWhiteRook` false)
    (set `self.WhiteRook` null)))

(event `self.WhiteBishopCollider.OnComponentBeginOverlap`
  (params (OverlappedComponent :type "PrimitiveComponent Object Reference") (OtherActor :type "Actor Object Reference") (OtherComp :type "PrimitiveComponent Object Reference") (OtherBodyIndex :type Integer) (bFromSweep :type Boolean) (SweepResult :type "HitResult Structure (by ref)"))
  ;[1 1 1] Chess piece has entered the right spot
  (if (== (`GameplayStatics.GetObjectClass` OtherActor) "/Game/Blueprints/Puzzles/MuralPuzzle/WhitePieces/BP_WhiteBishop.BP_WhiteBishop_C")
    (set `self.GotWhiteBishop` true)
    (set `self.WhiteBishop` OtherActor)))

(event `self.WhiteBishopCollider.OnComponentEndOverlap`
  (params (OverlappedComponent :type "PrimitiveComponent Object Reference") (OtherActor :type "Actor Object Reference") (OtherComp :type "PrimitiveComponent Object Reference") (OtherBodyIndex :type Integer))
  ;[1 1 1] Chess piece left its spot
  (if (== (`GameplayStatics.GetObjectClass` OtherActor) "/Game/Blueprints/Puzzles/MuralPuzzle/WhitePieces/BP_WhiteBishop.BP_WhiteBishop_C")
    (set `self.GotWhiteBishop` false)
    (set `self.WhiteBishop` null)))

(fn `UserConstructionScript`)