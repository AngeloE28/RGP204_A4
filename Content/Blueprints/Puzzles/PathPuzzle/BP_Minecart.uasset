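; BP_Minecart is the path puzzle minecart, a mesh driven by a hidden-mechanism physics body, MinecartMover.
; After the first overlap with the cart, Tick copies the mover's location, eases yaw toward its velocity and increases its mass above a height threshold.
; A looping timer toggles trail particles and the Moving flag by speed.
; That flag ramps audio volume, while pitch follows the player's time dilation.
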(event `self.ReceiveBeginPlay`
  ;[1 1 1] Begin play
  ;[1 1 1] Trail effects
  (`KismetSystemLibrary.K2_SetTimer` null "Trail" 0.05 true)
  ;[1 1 1] Gets the player
  (bind _returnvalue (`GameplayStatics.GetActorOfClass` "/Game/Player_BP/Blueprints/BP_Player.BP_Player_C"))
  (set `self.Player` _returnvalue)
  ;[1 1 1] Plays the sound
  (`AudioComponent.Play` (`self.Audio`) 0.0))

(event `SoundVolume`
  (bind _minvolume (`self.MinVolume`))
  (bind _maxvolume (`self.MaxVolume`))
  ;[1 1 1] Controls the volume of the sound
  (if (`self.Moving`)
    (`|MultiGate` false true
      (:`Out 0`
        (bind _output_get (set `self.CurrentVolume` (+ (`self.CurrentVolume`) (`self.VolumeIncrement`))))
        (if (>= _output_get _maxvolume)
          (set `self.CurrentVolume` _maxvolume))))
    (else
      (`|MultiGate` false true
        (:`Out 0`
          (bind _output_get_2 (set `self.CurrentVolume` (- (`self.CurrentVolume`) (`self.VolumeIncrement`))))
          (if (<= _output_get_2 _minvolume)
            (set `self.CurrentVolume` _minvolume)))))))

(event `self.ReceiveTick`
  (params (DeltaSeconds :type "Float (single-precision)"))
  (bind _minecartmover (`self.MinecartMover`))
  (bind _audio (`self.Audio`))
  ;[1 1 1] Event tick
  (`|ExecutionSequence`
    (:`then_0`
      ;[1 1 1] Sets the sound pitch
      (`AudioComponent.SetPitchMultiplier` _audio (`/Game/Player_BP/Blueprints/BP_Player.TotalTimeDilation` (`self.Player`)))
      (`self.SoundVolume`)
      (`AudioComponent.SetVolumeMultiplier` _audio (`self.CurrentVolume`)))
    (:`then_1`
      ;[1 1 1] Contrls the minecart mesh. Also changes minecart mover mass based on height
      (if (`self.Moved`)
        (`self.SetMinecartLocationAndRotation`)
        (if (> (.z (`SceneComponent.K2_GetComponentLocation` (`self.MinecartMover`))) 1630.0)
          (`PrimitiveComponent.SetMassOverrideInKg` _minecartmover "None" 1000.0 true)
          (else
            (`PrimitiveComponent.SetMassOverrideInKg` _minecartmover "None" 750.0 true)))))))

(event `SetMinecartLocationAndRotation`
  (bind _minecartmover (`self.MinecartMover`))
  (bind _minecart (`self.Minecart`))
  (bind _returnvalue (`SceneComponent.K2_GetComponentLocation` _minecartmover))
  ;[1 1 1] Sets the location and rotation of the minecart based on the ball that moves the minecart
  (`SceneComponent.K2_SetWorldLocation` (`self.Minecart`) _returnvalue false false)
  (`SceneComponent.K2_SetWorldRotation` _minecart (`KismetMathLibrary.RInterpTo` (`SceneComponent.K2_GetComponentRotation` _minecart) (`KismetMathLibrary.MakeRotator` 0.0 0.0 (.yaw (`KismetMathLibrary.FindLookAtRotation` _returnvalue (+ _returnvalue (`SceneComponent.GetComponentVelocity` _minecartmover))))) (`GameplayStatics.GetTimeSeconds`) (`self.InterpSpeed`)) false false))

(event `self.Minecart.OnComponentBeginOverlap`
  (params (OverlappedComponent :type "PrimitiveComponent Object Reference") (OtherActor :type "Actor Object Reference") (OtherComp :type "PrimitiveComponent Object Reference") (OtherBodyIndex :type Integer) (bFromSweep :type Boolean) (SweepResult :type "HitResult Structure (by ref)"))
  ;[1 1 1] Begin overlap minecart, sets the boolean moved to true
  (set `self.Moved` true))

(fn `Trail`
  (bind _particlesystem1 (`self.ParticleSystem1`))
  ;[1 1 1] Plays the particle system based on movement
  (bind _returnvalue (`PrimitiveComponent.GetPhysicsLinearVelocity` (`self.MinecartMover`) "None"))
  (if (>= (`KismetMathLibrary.VSize` _returnvalue) (`self.SpeedForParticles`))
    (`ActorComponent.Activate` _particlesystem1 false)
    (`ActorComponent.Activate` (`self.ParticleSystem`) false)
    (set `self.Moving` true)
    (else
      (`ActorComponent.Deactivate` _particlesystem1)
      (`ActorComponent.Deactivate` (`self.ParticleSystem`))
      (set `self.Moving` false))))

(fn `UserConstructionScript`)