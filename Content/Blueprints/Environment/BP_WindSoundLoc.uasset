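; BP_WindSoundLoc is a placeable environment zone that plays wind sound while the player is inside its collider.
; Overlap begin with BP_Player assigns WindSound to the audio component and plays it, and overlap end stops it and clears the sound.
; Every tick it sets the sound's pitch from the player's TotalTimeDilation, so the wind follows time dilation.
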(event `self.ReceiveBeginPlay`
  ;[1 1 1] Begin play
  ;[1 1 1] Gets the player
  (bind _returnvalue (`GameplayStatics.GetActorOfClass` "/Game/Player_BP/Blueprints/BP_Player.BP_Player_C"))
  (set `self.Player` _returnvalue))

(event `self.ReceiveTick`
  (params (DeltaSeconds :type "Float (single-precision)"))
  ;[1 1 1] Event tick
  ;[1 1 1] Sets the sound pitch
  (`AudioComponent.SetPitchMultiplier` (`self.Sound`) (`/Game/Player_BP/Blueprints/BP_Player.TotalTimeDilation` (`self.Player`))))

(event `self.Collider.OnComponentBeginOverlap`
  (params (OverlappedComponent :type "PrimitiveComponent Object Reference") (OtherActor :type "Actor Object Reference") (OtherComp :type "PrimitiveComponent Object Reference") (OtherBodyIndex :type Integer) (bFromSweep :type Boolean) (SweepResult :type "HitResult Structure (by ref)"))
  (bind _sound (`self.Sound`))
  ;[1 1 1] Begin overlap
  ;[1 1 1] Plays wind sound
  (if (== (`GameplayStatics.GetObjectClass` OtherActor) "/Game/Player_BP/Blueprints/BP_Player.BP_Player_C")
    (`AudioComponent.SetSound` _sound (`self.WindSound`))
    (`AudioComponent.Play` _sound 0.0)))

(event `self.Collider.OnComponentEndOverlap`
  (params (OverlappedComponent :type "PrimitiveComponent Object Reference") (OtherActor :type "Actor Object Reference") (OtherComp :type "PrimitiveComponent Object Reference") (OtherBodyIndex :type Integer))
  (bind _sound (`self.Sound`))
  ;[1 1 1] End overlap
  ;[1 1 1] Stops playing if player leaves the area by setting the sound to null
  (if (== (`GameplayStatics.GetObjectClass` OtherActor) "/Game/Player_BP/Blueprints/BP_Player.BP_Player_C")
    (`AudioComponent.Stop` _sound)
    (`AudioComponent.SetSound` _sound null)))

(fn `UserConstructionScript`)