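; BP_RopeTrap is a swinging-log trap that stays hidden until the player overlaps its trigger.
; Shooting the rope base breaks the constraints and cables, removes the kill collider and drops the log with physics.
; Touching the log collider spawns blood, makes the player drop a portal piece, disables dash, shoot and slow-time, and teleports them to the spawn point.
; The trap then resets by spawning a replacement and destroying itself.
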(event `self.ReceiveBeginPlay`
  ;[1 1 1] Beginplay
  ;[1 1 1] Gets the spawn point
  (bind _returnvalue (`GameplayStatics.GetActorOfClass` "/Game/Blueprints/Player/BP_SpawnPoint.BP_SpawnPoint_C"))
  (set `self.SpawnPoint` _returnvalue))

(event `self.RopeBase.OnComponentHit`
  (params (HitComponent :type "PrimitiveComponent Object Reference") (OtherActor :type "Actor Object Reference") (OtherComp :type "PrimitiveComponent Object Reference") (NormalImpulse :type "Vector Structure") (Hit :type "HitResult Structure (by ref)"))
  ;[1 1 1] Ropebase hit
  ;[1 1 1] Break trap event
  (if (== (`GameplayStatics.GetObjectClass` OtherActor) "/Game/Blueprints/Player/BP_Bullet.BP_Bullet_C")
    (`self.BreakTrap`)))

(event `BreakTrap`
  (bind _log (`self.Log`))
  ;[1 1 1] Breaks the trap
  (`PhysicsConstraintComponent.BreakConstraint` (`self.LeftBaseRope`))
  (`PhysicsConstraintComponent.BreakConstraint` (`self.RightBaseRope`))
  (set `CableComponent.bAttachEnd` false (`self.LeftBaseCable`))
  (set `CableComponent.bAttachEnd` false (`self.RightBaseCable`))
  (set `CableComponent.bAttachStart` false (`self.LeftRopeCable`))
  (set `CableComponent.bAttachStart` false (`self.RightRopeCable`))
  (`ActorComponent.K2_DestroyComponent` (`self.LogCollider`))
  (`SceneComponent.K2_DetachFromComponent` _log "KeepWorld" "KeepWorld" "KeepWorld" true)
  (`PrimitiveComponent.SetCollisionEnabled` _log "PhysicsOnly")
  (`PrimitiveComponent.SetSimulatePhysics` _log true))

(event `self.TrapTrigger.OnComponentBeginOverlap`
  (params (OverlappedComponent :type "PrimitiveComponent Object Reference") (OtherActor :type "Actor Object Reference") (OtherComp :type "PrimitiveComponent Object Reference") (OtherBodyIndex :type Integer) (bFromSweep :type Boolean) (SweepResult :type "HitResult Structure (by ref)"))
  ;[1 1 1] Trap Trigger Overlap
  ;[1 1 1] Activates the trap
  (if (== (`GameplayStatics.GetObjectClass` OtherActor) "/Game/Player_BP/Blueprints/BP_Player.BP_Player_C")
    (`self.ActivateTrap`)))

(event `ActivateTrap`
  ;[1 1 1] Activates the trap
  (`SceneComponent.SetHiddenInGame` (`self.RopeBase`) false true)
  (`SceneComponent.SetHiddenInGame` (`self.Base`) false true)
  (`SceneComponent.SetHiddenInGame` (`self.Log`) false true)
  (`SceneComponent.SetHiddenInGame` (`self.LogCollider`) true false)
  (`ActorComponent.K2_DestroyComponent` (`self.SpikeHolder`))
  (`ActorComponent.K2_DestroyComponent` (`self.Front`))
  (`ActorComponent.K2_DestroyComponent` (`self.Back`)))

(event `self.LogCollider.OnComponentBeginOverlap`
  (params (OverlappedComponent :type "PrimitiveComponent Object Reference") (OtherActor :type "Actor Object Reference") (OtherComp :type "PrimitiveComponent Object Reference") (OtherBodyIndex :type Integer) (bFromSweep :type Boolean) (SweepResult :type "HitResult Structure (by ref)"))
  (bind _sphere (`/Game/Blueprints/Player/BP_SpawnPoint.Sphere` (`self.SpawnPoint`)))
  ;[1 1 1] SpikeCollider Overlap
  ;[1 1 1] Teleports player to the checkpoint and resets the trap
  (if (== (`GameplayStatics.GetObjectClass` OtherActor) "/Game/Player_BP/Blueprints/BP_Player.BP_Player_C")
    (`NiagaraFunctionLibrary.SpawnSystemAtLocation` (`self.NS_BloodSplat`) (`self.K2_GetActorLocation` OtherActor))
    (bind _asbp_player (cast `/Game/Player_BP/Blueprints/BP_Player` OtherActor))
    (`|ExecutionSequence`
      (:`then_0`
        (`/Game/Player_BP/Blueprints/BP_Player.DropPortalPiece` _asbp_player))
      (:`then_1`
        (set `/Game/Player_BP/Blueprints/BP_Player.canDash` false _asbp_player))
      (:`then_2`
        (set `/Game/Player_BP/Blueprints/BP_Player.canShoot` false _asbp_player))
      (:`then_3`
        (set `/Game/Player_BP/Blueprints/BP_Player.canSlowTime` false _asbp_player))
      (:`then_4`
        (`self.K2_TeleportTo` _asbp_player (`SceneComponent.K2_GetComponentLocation` _sphere) (`SceneComponent.K2_GetComponentRotation` _sphere))
        (bind _returnvalue (`|SpawnActorFromClass` "BP_RopeTrap_C" (`SceneComponent.K2_GetComponentToWorld` (`self.DefaultSceneRoot`)) "Undefined" "OverrideRootScale" null null))
        (`SceneComponent.K2_SetWorldTransform` (`/Game/Blueprints/Traps/BP_RopeTrap.TrapTrigger` _returnvalue) (`SceneComponent.K2_GetComponentToWorld` (`self.TrapTrigger`)) false false)
        (`self.K2_DestroyActor`)))))

(fn `UserConstructionScript`)