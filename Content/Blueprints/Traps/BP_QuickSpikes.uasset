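; BP_QuickSpikes is a trap that sends the player back to the spawn point on contact.
; On BeginPlay it caches the BP_SpawnPoint, then plays a timeline at a configurable rate, lerping the sword pivot between two marker positions.
; When the sword mesh overlaps BP_Player, the player drops the key, loses dash, shoot and slow-time abilities, and teleports to the spawn point's sphere.
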(event `self.ReceiveBeginPlay`
  ;[1 1 1] Beginplay
  (`|ExecutionSequence`
    (:`then_0`
      ;[1 1 1] Gets the spawn point
      (bind _returnvalue (`GameplayStatics.GetActorOfClass` "/Game/Blueprints/Player/BP_SpawnPoint.BP_SpawnPoint_C"))
      (set `self.SpawnPoint` _returnvalue))
    (:`then_1`
      ;[1 1 1] Runs the move spike event
      (`self.MoveSpike`))))

(event `MoveSpike`
  ;[1 1 1] Moves the sword
  (set `self.Position1` (`SceneComponent.K2_GetComponentLocation` (`self.Pos1`)))
  (set `self.Position2` (`SceneComponent.K2_GetComponentLocation` (`self.Pos2`)))
  (`TimelineComponent.SetPlayRate` (`self.Move`) (`self.PlayRate`))
  (bind (_direction _alpha) (`Timeline|Move`)
    (:`Update`
      (`SceneComponent.K2_SetWorldLocation` (`self.SwordTingPivot`) (`KismetMathLibrary.VLerp` (`self.Position1`) (`self.Position2`) _alpha) false false))))

(event `self.SwordTing.OnComponentBeginOverlap`
  (params (OverlappedComponent :type "PrimitiveComponent Object Reference") (OtherActor :type "Actor Object Reference") (OtherComp :type "PrimitiveComponent Object Reference") (OtherBodyIndex :type Integer) (bFromSweep :type Boolean) (SweepResult :type "HitResult Structure (by ref)"))
  (bind _sphere (`/Game/Blueprints/Player/BP_SpawnPoint.Sphere` (`self.SpawnPoint`)))
  ;[1 1 1] Begin overlap
  ;[1 1 1] Teleports player to the checkpoint
  (if (== (`GameplayStatics.GetObjectClass` OtherActor) "/Game/ThirdPersonBP/Blueprints/BP_Player.BP_Player_C")
    (bind _asbp_player (cast `/Game/ThirdPersonBP/Blueprints/BP_Player` OtherActor))
    (`|ExecutionSequence`
      (:`then_0`
        (`/Game/ThirdPersonBP/Blueprints/BP_Player.DropKey` _asbp_player))
      (:`then_1`
        (set `/Game/ThirdPersonBP/Blueprints/BP_Player.canDash` false _asbp_player))
      (:`then_2`
        (set `/Game/ThirdPersonBP/Blueprints/BP_Player.canShoot` false _asbp_player))
      (:`then_3`
        (set `/Game/ThirdPersonBP/Blueprints/BP_Player.canSlowTime` false _asbp_player))
      (:`then_4`
        (`self.K2_TeleportTo` _asbp_player (`SceneComponent.K2_GetComponentLocation` _sphere) (`SceneComponent.K2_GetComponentRotation` _sphere))))))

(fn `UserConstructionScript`)