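; BP_CheckPoint is a checkpoint actor that updates where the player respawns.
; On BeginPlay it finds the level's BP_SpawnPoint and caches it.
; When a BP_Player overlaps its static mesh, it teleports that spawn point to the location and rotation of its SpawnPointPos component, rather than storing a separate respawn transform.
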(event `self.ReceiveBeginPlay`
  ;[1 1 1] Gets the spawn point
  (bind _returnvalue (`GameplayStatics.GetActorOfClass` "/Game/Blueprints/Player/BP_SpawnPoint.BP_SpawnPoint_C"))
  (set `self.SpawnPoint` _returnvalue))

(event `self.StaticMeshComponent.OnComponentBeginOverlap`
  (params (OverlappedComponent :type "PrimitiveComponent Object Reference") (OtherActor :type "Actor Object Reference") (OtherComp :type "PrimitiveComponent Object Reference") (OtherBodyIndex :type Integer) (bFromSweep :type Boolean) (SweepResult :type "HitResult Structure (by ref)"))
  (bind _spawnpointpos (`self.SpawnPointPos`))
  ;[1 1 1] Creates a checkpoint for the player
  (if (== (`GameplayStatics.GetObjectClass` OtherActor) "/Game/ThirdPersonBP/Blueprints/BP_Player.BP_Player_C")
    (`self.K2_TeleportTo` (`self.SpawnPoint`) (`SceneComponent.K2_GetComponentLocation` _spawnpointpos) (`SceneComponent.K2_GetComponentRotation` _spawnpointpos))))

(fn `UserConstructionScript`)