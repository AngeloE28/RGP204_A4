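; BP_Bullet is a player bullet actor that reacts to whatever it hits.
; On Hit, it pushes physics-simulating components with an impulse scaled from its own velocity, applied at the bullet's location.
; On any hit, it then destroys itself and spawns the BulletExplosion particle system there, oriented opposite its forward vector.
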(event `self.ReceiveHit`
  (params (MyComp :type "PrimitiveComponent Object Reference") (Other :type "Actor Object Reference") (OtherComp :type "PrimitiveComponent Object Reference") (bSelfMoved :type Boolean) (HitLocation :type "Vector Structure") (HitNormal :type "Vector Structure") (NormalImpulse :type "Vector Structure") (Hit :type "HitResult Structure (by ref)"))
  (bind _returnvalue (`self.K2_GetActorLocation`))
  ;[1 1 1] Adds impulse to physics object hit
  (if (`SceneComponent.IsSimulatingPhysics` OtherComp "None")
    (`PrimitiveComponent.AddImpulseAtLocation` OtherComp (* (`self.GetVelocity`) 100.0) _returnvalue "None"))
  (`self.K2_DestroyActor`)
  (`NiagaraFunctionLibrary.SpawnSystemAtLocation` "/Game/Effects/BulletExplosion.BulletExplosion" _returnvalue (`KismetMathLibrary.Conv_VectorToRotator` (* (`self.GetActorForwardVector`) -1.0))))

(fn `UserConstructionScript`)