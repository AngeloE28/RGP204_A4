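; BP_GhostTrails is a ghost trail actor that shows a frozen afterimage of the player's current pose.
; On BeginPlay it gives each PoseableMesh material slot a dynamic ghost material, copies the player mesh's pose and starts the Opacity timeline.
; The timeline's update logic, marked as never run, would set a material scalar (parameter name None) and destroy the actor after DestroyTimer.
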(event `self.ReceiveBeginPlay`
  ;[1 1 1] Begin Play
  (bind _asbp_player (cast `/Game/ThirdPersonBP/Blueprints/BP_Player` (`GameplayStatics.GetPlayerPawn` 0)))
  (set `self.PlayerRef` _asbp_player)
  (`self.GhostTrails`))

(event `GhostTrails`
  ;[1 1 1] Creates a ghost trail
  (for _ (`MeshComponent.GetMaterials` (`self.PoseableMesh`))
    (bind _returnvalue (`KismetMaterialLibrary.CreateDynamicMaterialInstance` "/Game/Materials/GhostTrailMat_Inst.GhostTrailMat_Inst"))
    (bind _returnvalue_2 (`KismetArrayLibrary.Array_Add` (`self.DynamicMaterials`) _returnvalue))
    (`PrimitiveComponent.SetMaterial` (`self.PoseableMesh`) _returnvalue_2 _returnvalue)
    (`PoseableMeshComponent.CopyPoseFromSkeletalComponent` (`self.PoseableMesh`) (`Character.Mesh` (`self.PlayerRef`)))
    (`TimelineComponent.PlayFromStart` (`self.Opacity`))))

(fn `UserConstructionScript`
  (`KismetArrayLibrary.Array_Clear` (`self.DynamicMaterials`)))